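; Procedural dungeon generator actor that spawns a starting room and one random connected room on BeginPlay.
; It places BP_Dungeon_Room_1 at its root transform and gathers the child components of that room's ExitsFolder as exit points.
; A random class from RoomList then spawns at a randomly chosen exit's location and rotation.
; That room is cast to BP_Master_Room and stored as LatestRoom.
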(event Custom|SpawnStartRoom
  ;[0.027 1 0.1503 1 30] Spawn Starting Room
  (bind _returnvalue (Game|SpawnActorfromClass "/Game/Procedural_Dungeon/BP_Dungeon_Room_1.BP_Dungeon_Room_1_C" (Transformation|GetWorldTransform (Variables|Default|GetDefaultSceneRoot)) "AlwaysSpawn" "MultiplyWithRoot" 0 0))
  (Utilities|Array|AppendArray (Variables|Default|GetExitsList) (Components|GetChildrenComponents (Variables|/Game/Procedural_Dungeon/BP_Master_Room.BP_Master_Room_C|GetExitsFolder _returnvalue) false)))

(event Custom|SpawnNextRoom
  (Variables|Default|SetSelectedExitPoint (.OutItem (Utilities|Array|Random (Variables|Default|GetExitsList))))
  (bind _returnvalue (Game|SpawnActorfromClass (.OutItem (Utilities|Array|Random (Variables|Default|GetRoomList))) (Math|Transform|MakeTransform (Transformation|GetWorldLocation (Variables|Default|GetSelectedExitPoint)) (Transformation|GetWorldRotation (Variables|Default|GetSelectedExitPoint)) "1.000000,1.000000,1.000000") "AlwaysSpawn" "MultiplyWithRoot" 0 0))
  (bind _asbp_master_room (Utilities|Casting|CastToBP_Master_Room _returnvalue))
  (Variables|Default|SetLatestRoom _asbp_master_room))

(event EventBeginPlay
  (CallFunction|SpawnStartRoom)
  (CallFunction|SpawnNextRoom))

(fn ConstructionScript)