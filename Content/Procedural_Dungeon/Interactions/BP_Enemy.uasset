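; Enemy AI for the procedural dungeon that wanders the navmesh, chases players and resets any it catches to a fixed location.
; A self-restarting AIMoveTo loop either picks random reachable points, spawning an AI_Destination at each, or follows the tagged player.
; Proximity overlaps toggle chasing and walk speed, which is slower during a chase.
; Box overlap teleports the player, adds a Niagara component and plays a sound.
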(event OnComponentBeginOverlap(Proximity)
  (params (OverlappedComponent :type Primitive%20Component%20Object%20Reference) (OtherActor :type Actor%20Object%20Reference) (OtherComp :type Primitive%20Component%20Object%20Reference) (OtherBodyIndex :type Integer) (bFromSweep :type Boolean) (SweepResult :type Hit%20Result%20Structure%20%28by%20ref%29))
  ;[0.02732 1 0.15 1 30] Enemy AI
  (if (Actor|ActorHasTag OtherActor "Player")
    (Variables|Default|SetOther%20Actor OtherActor)
    (Variables|Default|SetIs%20Chasing true)
    (Variables|/Script/Engine.CharacterMovementComponent|SetMaxWalkSpeed (Variables|Character|GetCharacterMovement) 3e+02)
    (CallFunction|CheckforPlayers)))

(event OnComponentEndOverlap(Proximity)
  (params (OverlappedComponent :type Primitive%20Component%20Object%20Reference) (OtherActor :type Actor%20Object%20Reference) (OtherComp :type Primitive%20Component%20Object%20Reference) (OtherBodyIndex :type Integer))
  ;[0.02732 1 0.15 1 30] Enemy AI
  (if (Actor|ActorHasTag OtherActor "Player")
    (Variables|Default|SetIs%20Chasing false)
    (Variables|/Script/Engine.CharacterMovementComponent|SetMaxWalkSpeed (Variables|Character|GetCharacterMovement) 5e+02)
    (CallFunction|CheckforPlayers)))

(event OnComponentBeginOverlap(Box)
  (params (OverlappedComponent :type Primitive%20Component%20Object%20Reference) (OtherActor :type Actor%20Object%20Reference) (OtherComp :type Primitive%20Component%20Object%20Reference) (OtherBodyIndex :type Integer) (bFromSweep :type Boolean) (SweepResult :type Hit%20Result%20Structure%20%28by%20ref%29))
  ;[0 1 0.1582 1 30] Resetting Players
  (if (Actor|ActorHasTag OtherActor "Player")
    (bind _asbp_third_person_character (Utilities|Casting|CastToBP_ThirdPersonCharacter OtherActor))
    (Transformation|SetActorLocationAndRotation _asbp_third_person_character "-697.782025,-0.000017,379.260574")
    (AddComponent|AddNiagaraComponent _asbp_third_person_character false (Transformation|GetRelativeTransform (Variables|/Script/Engine.Character|GetMesh _asbp_third_person_character)))
    (Audio|SpawnSound2D "/Engine/EditorSounds/Notifications/CompileFailed_Cue.CompileFailed_Cue" 1.0 1.0 0.0 0)))

(event Custom|Check%20for%20Players
  ;[0.02732 1 0.15 1 30] Enemy AI
  (if (Variables|Default|GetIs%20Chasing)
    (AI|AIMoveTo self "0, 0, 0" (Variables|Default|GetOther%20Actor) 5.0 false
      (:OnSuccess
        _)
      (:OnFail
        _))
    (CallFunction|CheckforPlayers)
    (else
      (bind _randomlocation (Class|NavigationSystemV1|GetRandomLocationinNavigableRadius (Transformation|GetActorLocation) 2e+03 0 0))
      (Game|SpawnActorfromClass "/Game/Procedural_Dungeon/Interactions/AI_Destination.AI_Destination_C" (Math|Transform|MakeTransform _randomlocation "0, 0, 0" "1.000000,1.000000,1.000000") "AlwaysSpawn" "MultiplyWithRoot" 0 0)
      (AI|AIMoveTo self _randomlocation 0 5.0 false
        (:OnSuccess
          _)
        (:OnFail
          _))
      (CallFunction|CheckforPlayers))))

(event EventBeginPlay
  ;[0.02732 1 0.15 1 30] Enemy AI
  (CallFunction|CheckforPlayers))

(fn ConstructionScript)